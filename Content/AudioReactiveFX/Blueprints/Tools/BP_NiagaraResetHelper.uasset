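; BP_NiagaraResetHelper is a utility actor that restarts every Niagara component on all actors in the level.
; FixNiagara loops through each actor's Niagara components, calling either ReinitializeSystem or ResetSystem depending on the FullReinitialize flag.
; With AutoFix enabled, it runs on BeginPlay, and the construction script also sets a short one-shot timer.
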(event EventBeginPlay
  (if (Variables|Default|GetAutoFix)
    (CallFunction|FixNiagara)))

(event Collision|EventActorBeginOverlap
  (params (OtherActor :type Actor%20Object%20Reference)))

(event EventTick
  (params (DeltaSeconds :type Float%20%28single-precision%29)))

(fn ConstructionScript
  (if (Variables|Default|GetAutoFix)
    (Utilities|Time|SetTimerbyEvent (EventDispatchers|CreateEvent :!event FixNiagara) 0.5)))

(fn FixNiagara
  (bind _outactors (Actor|GetAllActorsOfClass "/Script/Engine.Actor"))
  (for _array_element _outactors
    (for _array_element_2 (Actor|GetComponentsByClass _array_element "/Script/Niagara.NiagaraComponent")
      (if (Variables|Default|GetFullReinitialize)
        (Niagara|ReinitializeSystem _array_element_2)
        (else
          (Niagara|ResetSystem _array_element_2))))))